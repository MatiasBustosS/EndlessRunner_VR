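; BP_Coleccionable is a collectible pickup that destroys itself when a ThirdPersonCharacter overlaps its Box component, with no reward logic connected.
; Every Tick it also compares its world X with player 0's character and, once the player's X is greater, destroys itself after a short Delay.
; A cast to ThirdPersonGameMode is left unwired and never runs.
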(event OnComponentBeginOverlap(Box)
  (params (OverlappedComponent :type Primitive%20Component%20Object%20Reference) (OtherActor :type Actor%20Object%20Reference) (OtherComp :type Primitive%20Component%20Object%20Reference) (OtherBodyIndex :type Integer) (bFromSweep :type Boolean) (SweepResult :type Hit%20Result%20Structure%20%28by%20ref%29))
  (Utilities|Casting|CastToThirdPersonCharacter OtherActor)
  (Actor|DestroyActor))

(event EventTick
  (params (DeltaSeconds :type Float%20%28single-precision%29))
  (bind _asthird_person_character (Utilities|Casting|CastToThirdPersonCharacter (Game|GetPlayerCharacter 0)))
  (if (< (.x (Transformation|GetActorLocation)) (.x (Transformation|GetActorLocation _asthird_person_character)))
    (Utilities|FlowControl|Delay 1.5)
    (Actor|DestroyActor)))

(fn ConstructionScript)
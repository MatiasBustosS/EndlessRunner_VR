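; Road segment actor that populates itself with obstacles and pickups, then removes itself after the player passes through.
; On BeginPlay it occasionally spawns a jump or dash power-up, then randomly picks a preset layout of barriers, coins and diamonds at arrow markers, with one roll leaving that layout empty.
; When ThirdPersonCharacter overlaps DestroyBox, the segment destroys itself after a short delay, without explicitly destroying what it spawned.
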(event OnComponentBeginOverlap(DestroyBox)
  (params (OverlappedComponent :type Primitive%20Component%20Object%20Reference) (OtherActor :type Actor%20Object%20Reference) (OtherComp :type Primitive%20Component%20Object%20Reference) (OtherBodyIndex :type Integer) (bFromSweep :type Boolean) (SweepResult :type Hit%20Result%20Structure%20%28by%20ref%29))
  (Utilities|Casting|CastToThirdPersonCharacter OtherActor)
  (Utilities|FlowControl|Delay 2.0)
  (Actor|DestroyActor))

(event EventBeginPlay
  (CallFunction|SpawnPowerUp)
  (CallFunction|SpawnwithCoin))

(fn ConstructionScript)

(fn SpawnwithCoin
  (switch int (Math|Random|RandomIntegerinRange 0 6)
    (:0
      (Game|SpawnActorfromClass "/Game/Obstaculo/BP_Barrera.BP_Barrera_C" (Transformation|GetWorldTransform (Variables|Default|GetArrow0)) "Undefined" 0 0)
      (Game|SpawnActorfromClass "/Game/Obstaculo/BP_Barrera.BP_Barrera_C" (Transformation|GetWorldTransform (Variables|Default|GetArrow1)) "Undefined" 0 0)
      (Game|SpawnActorfromClass "/Game/Collectinable/BP_Coin.BP_Coin_C" (Transformation|GetWorldTransform (Variables|Default|Getc_2)) "Undefined" 0 0)
      (Game|SpawnActorfromClass "/Game/Obstaculo/BP_Barrera.BP_Barrera_C" (Transformation|GetWorldTransform (Variables|Default|GetArrow3)) "Undefined" 0 0)
      (Game|SpawnActorfromClass "/Game/Obstaculo/BP_Barrera.BP_Barrera_C" (Transformation|GetWorldTransform (Variables|Default|GetArrow5)) "Undefined" 0 0)
      (Game|SpawnActorfromClass "/Game/Collectinable/BP_Coin.BP_Coin_C" (Transformation|GetWorldTransform (Variables|Default|Getc_4)) "Undefined" 0 0))
    (:1
      (Game|SpawnActorfromClass "/Game/Obstaculo/BP_Barrera.BP_Barrera_C" (Transformation|GetWorldTransform (Variables|Default|GetArrow3)) "Undefined" 0 0)
      (Game|SpawnActorfromClass "/Game/Obstaculo/BP_Barrera.BP_Barrera_C" (Transformation|GetWorldTransform (Variables|Default|GetArrow5)) "Undefined" 0 0)
      (Game|SpawnActorfromClass "/Game/Collectinable/BP_Diamond.BP_Diamond_C" (Transformation|GetWorldTransform (Variables|Default|Getc_4)) "Undefined" 0 0)
      (Game|SpawnActorfromClass "/Game/Obstaculo/BP_Barrera.BP_Barrera_C" (Transformation|GetWorldTransform (Variables|Default|GetArrow1)) "Undefined" 0 0)
      (Game|SpawnActorfromClass "/Game/Obstaculo/BP_Barrera.BP_Barrera_C" (Transformation|GetWorldTransform (Variables|Default|GetArrow2)) "Undefined" 0 0)
      (Game|SpawnActorfromClass "/Game/Collectinable/BP_Coin.BP_Coin_C" (Transformation|GetWorldTransform (Variables|Default|Getc_0)) "Undefined" 0 0))
    (:2
      (Game|SpawnActorfromClass "/Game/Obstaculo/BP_Barrera.BP_Barrera_C" (Transformation|GetWorldTransform (Variables|Default|GetArrow4)) "Undefined" 0 0)
      (Game|SpawnActorfromClass "/Game/Obstaculo/BP_Barrera.BP_Barrera_C" (Transformation|GetWorldTransform (Variables|Default|GetArrow5)) "Undefined" 0 0)
      (Game|SpawnActorfromClass "/Game/Collectinable/BP_Coin.BP_Coin_C" (Transformation|GetWorldTransform (Variables|Default|Getc_3)) "Undefined" 0 0)
      (Game|SpawnActorfromClass "/Game/Obstaculo/BP_Barrera.BP_Barrera_C" (Transformation|GetWorldTransform (Variables|Default|GetArrow0)) "Undefined" 0 0)
      (Game|SpawnActorfromClass "/Game/Obstaculo/BP_Barrera.BP_Barrera_C" (Transformation|GetWorldTransform (Variables|Default|GetArrow1)) "Undefined" 0 0)
      (Game|SpawnActorfromClass "/Game/Collectinable/BP_Coin.BP_Coin_C" (Transformation|GetWorldTransform (Variables|Default|Getc_2)) "Undefined" 0 0))
    (:3
      (Game|SpawnActorfromClass "/Game/Obstaculo/BP_Barrera.BP_Barrera_C" (Transformation|GetWorldTransform (Variables|Default|GetArrow1)) "Undefined" 0 0)
      (Game|SpawnActorfromClass "/Game/Obstaculo/BP_Barrera.BP_Barrera_C" (Transformation|GetWorldTransform (Variables|Default|GetArrow2)) "Undefined" 0 0)
      (Game|SpawnActorfromClass "/Game/Collectinable/BP_Coin.BP_Coin_C" (Transformation|GetWorldTransform (Variables|Default|Getc_0)) "Undefined" 0 0)
      (Game|SpawnActorfromClass "/Game/Obstaculo/BP_Barrera.BP_Barrera_C" (Transformation|GetWorldTransform (Variables|Default|GetArrow3)) "Undefined" 0 0)
      (Game|SpawnActorfromClass "/Game/Obstaculo/BP_Barrera.BP_Barrera_C" (Transformation|GetWorldTransform (Variables|Default|GetArrow5)) "Undefined" 0 0)
      (Game|SpawnActorfromClass "/Game/Collectinable/BP_Coin.BP_Coin_C" (Transformation|GetWorldTransform (Variables|Default|Getc_4)) "Undefined" 0 0))
    (:4
      (Game|SpawnActorfromClass "/Game/Obstaculo/BP_Barrera.BP_Barrera_C" (Transformation|GetWorldTransform (Variables|Default|GetArrow6)) "Undefined" 0 0)
      (Game|SpawnActorfromClass "/Game/Obstaculo/BP_Barrera.BP_Barrera_C" (Transformation|GetWorldTransform (Variables|Default|GetArrow7)) "Undefined" 0 0)
      (Game|SpawnActorfromClass "/Game/Obstaculo/BP_Barrera.BP_Barrera_C" (Transformation|GetWorldTransform (Variables|Default|GetArrow3)) "Undefined" 0 0)
      (Game|SpawnActorfromClass "/Game/Obstaculo/BP_Barrera.BP_Barrera_C" (Transformation|GetWorldTransform (Variables|Default|GetArrow5)) "Undefined" 0 0)
      (Game|SpawnActorfromClass "/Game/Collectinable/BP_Coin.BP_Coin_C" (Transformation|GetWorldTransform (Variables|Default|Getc_4)) "Undefined" 0 0)
      (Game|SpawnActorfromClass "/Game/Collectinable/BP_Diamond.BP_Diamond_C" (Transformation|GetWorldTransform (Variables|Default|Getc_0)) "Undefined" 0 0))
    (:5
      (Game|SpawnActorfromClass "/Game/Obstaculo/BP_Barrera.BP_Barrera_C" (Transformation|GetWorldTransform (Variables|Default|GetArrow0)) "Undefined" 0 0)
      (Game|SpawnActorfromClass "/Game/Obstaculo/BP_Barrera.BP_Barrera_C" (Transformation|GetWorldTransform (Variables|Default|GetArrow2)) "Undefined" 0 0)
      (Game|SpawnActorfromClass "/Game/Collectinable/BP_Diamond.BP_Diamond_C" (Transformation|GetWorldTransform (Variables|Default|Getc_1)) "Undefined" 0 0)
      (Game|SpawnActorfromClass "/Game/Obstaculo/BP_Barrera.BP_Barrera_C" (Transformation|GetWorldTransform (Variables|Default|GetArrow4)) "Undefined" 0 0)
      (Game|SpawnActorfromClass "/Game/Obstaculo/BP_Barrera.BP_Barrera_C" (Transformation|GetWorldTransform (Variables|Default|GetArrow5)) "Undefined" 0 0)
      (Game|SpawnActorfromClass "/Game/Collectinable/BP_Coin.BP_Coin_C" (Transformation|GetWorldTransform (Variables|Default|Getc_3)) "Undefined" 0 0))))

(fn SpawnPowerUp
  (switch int (Math|Random|RandomIntegerinRange 0 10)
    (:3
      (Game|SpawnActorfromClass "/Game/PowerUp/PowerUp_Jump.PowerUp_Jump_C" (Transformation|GetWorldTransform (Variables|Default|GetArrow8)) "Undefined" 0 0))
    (:8
      (Game|SpawnActorfromClass "/Game/PowerUp/PowerUp_Dash.PowerUp_Dash_C" (Transformation|GetWorldTransform (Variables|Default|GetArrow8)) "Undefined" 0 0))))